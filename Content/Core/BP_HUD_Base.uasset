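; BP_HUD_Base is a HUD Blueprint that manages the on-screen interaction prompt showing an actor's name.
; On BeginPlay it creates the interact widget for player 0, adds it to the viewport and hides it.
; DrawHUD caches the screen size, which the show event uses to position the widget at screen center after setting its name text.
; Showing also prints a Russian debug message; a separate event hides the widget.
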(event `self.ReceiveBeginPlay`
  (`self.Event Create Interact Widget`))

(event `self.ReceiveDrawHUD`
  (params (SizeX :type Integer) (SizeY :type Integer))
  (set `self.Size X` SizeX)
  (set `self.Size Y` SizeY))

(event `Event Create Interact Widget`
  ;[0.15 0.15 0.15 0.5 50] Interact Widget
  (bind _returnvalue (`|CreateWidget` (`self.Interact Widget Ref`) (`GameplayStatics.GetPlayerController` 0)))
  (bind _output_get (set `self.Interact Widget` _returnvalue))
  (`UserWidget.AddToViewport` _output_get 0)
  (`Widget.SetVisibility` _output_get "Hidden"))

(event `/Game/Core/Interfaces/BPI_HUD.Update_And_Show_Interact_Widget`
  (params (`Actor Name` :type Name))
  (bind _interact_widget (`self.Interact Widget`))
  ;[0.15 0.15 0.15 0.5 50] Interact Widget
  (set `TextBlock.Text` (`KismetTextLibrary.Conv_NameToText` `Actor Name`) (`/Game/Core/UI/WBP_Interact.ObjectNameText` _interact_widget))
  (`UserWidget.SetPositionInViewport` _interact_widget (`KismetMathLibrary.MakeVector2D` (`KismetMathLibrary.Conv_IntToDouble` (/ (`self.Size X`) 2)) (`KismetMathLibrary.Conv_IntToDouble` (/ (`self.Size Y`) 2))) true)
  (`Widget.SetVisibility` _interact_widget "HitTestInvisible")
  (`KismetSystemLibrary.PrintString` "Имя актора принято в виджет!" true true (struct :`R` 0.105079 :`G` 0.260603 :`B` 0.637597 :`A` 1.0) 15.0))

(event `/Game/Core/Interfaces/BPI_HUD.Hidden_Interact_Widget`
  ;[0.15 0.15 0.15 0.5 50] Interact Widget
  (`Widget.SetVisibility` (`self.Interact Widget`) "Hidden"))

(fn `UserConstructionScript`)