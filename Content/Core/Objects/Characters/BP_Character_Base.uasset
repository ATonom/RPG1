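; Base character Blueprint that executes broadcast commands for movement, rotation, camera zoom and a world cursor, and exposes movement state getters.
; On BeginPlay it binds health component events (destroying itself when health empties), detects player control, requests the HUD and adds a Stigmat component.
; Overlaps focus one BPI_Interactable actor at a time for interaction, with players relaying its name to the HUD through BPI_HUD.
; A temporary hit input applies test damage.
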(event `self.ReceiveBeginPlay`
  (`|ExecutionSequence`
    (:`then_0`
      ;[0.15 0.15 0.15 0.502 100] Хелз компонент
      (bind _bp_healthcomponent (`self.BP_HealthComponent`)
        (:`then`
          (add `/Game/Core/Components/BP_Health_Component.Event On Health Empty` _bp_healthcomponent (delegate `Event On Health Empty_Event`))
          ;;[0.1144 0.3005 0.8879 1 100] Тест
          (add `/Game/Core/Components/BP_Health_Component.Event On Health Change` _bp_healthcomponent (delegate `Event On Health Change_Event`)) ; Подписываемся на изменение HP Хелз компонента
        )
        (:`else`)))
    (:`then_1`
      (`self.Setup Character`))))

(event `EnhancedInput|/Game/Core/Input/Actions/IA_Hit`
  (params (ActionValue :type Boolean) (ElapsedSeconds :type "Float (double-precision)") (TriggeredSeconds :type "Float (double-precision)") (InputAction :type "InputAction Object Reference" :default "/Game/Core/Input/Actions/IA_Hit.IA_Hit"))
  ;[0.15 0.15 0.15 0.502 100] Хелз компонент
  ;;[0.1144 0.3005 0.8879 1 100] Тест
  (:`Started`
    (bind _bp_healthcomponent (`self.BP_HealthComponent`)
      (:`then`
        (`/Game/Core/Components/BP_Health_Component.Recaive Damage` _bp_healthcomponent 25.0))
      (:`else`))))

(event `Event On Health Change_Event`
  (params (`Current Health` :type "Float (double-precision)"))
  ;[0.15 0.15 0.15 0.502 100] Хелз компонент
  ;;[0.1144 0.3005 0.8879 1 100] Тест
  (`KismetSystemLibrary.PrintString` (`KismetStringLibrary.Conv_DoubleToString` `Current Health`)))

(event `Event On Health Empty_Event`
  ;[0.15 0.15 0.15 0.502 100] Хелз компонент
  (`self.K2_DestroyActor`))

(event `self.ReceiveActorBeginOverlap`
  (params (OtherActor :type "Actor Object Reference"))
  ;[0.15 0.15 0.15 0.5 100] Event ActorBeginOverlap
  (`/Engine/EditorBlueprintResources/StandardMacros.IsValid` OtherActor
    (:`Is Valid`
      (`|ExecutionSequence`
        (:`then_0`
          (if (not (`self.bFocused To Interact Actor`))
            (if (`KismetSystemLibrary.DoesImplementInterface` OtherActor "/Game/Core/Interfaces/BPI_Interactable.BPI_Interactable_C")
              (set `self.bFocused To Interact Actor` true)
              (bind _output_get (set `self.Actor Of Interaction` OtherActor))
              (message `/Game/Core/Interfaces/BPI_Interactable.Request_Actor_Name` _output_get self)
              (`KismetSystemLibrary.PrintString` "Найден предмет!  Запрос имени." true true (struct :`R` 0.991102 :`G` 0.113312 :`B` 0.156393 :`A` 1.0) 15.0))
            (else
              (`KismetSystemLibrary.PrintString` "Игрок уже взаимодействует!" true true (struct :`R` 0.991102 :`G` 0.113312 :`B` 0.156393 :`A` 1.0) 15.0))))))))

(event `/Game/Core/Interfaces/BPI_Inputs.Broadcast_Char_Rotation`
  (params (`New Rotation Z (Yaw)` :type "Float (double-precision)"))
  ;[0.15 0.15 0.15 0.5 100] Поворот персонажа
  (`self.K2_SetActorRotation` (`KismetMathLibrary.MakeRotator` 0.0 0.0 `New Rotation Z (Yaw)`)))

(event `/Game/Core/Interfaces/BPI_Inputs.Broadcast_Move`
  (params (`Value X` :type "Float (double-precision)") (`Value Y` :type "Float (double-precision)") (`Value Z` :type "Float (double-precision)"))
  ;[0.15 0.15 0.15 0.5 100] Передвижение
  (`self.AddMovementInput` (`KismetMathLibrary.MakeVector` `Value X` `Value Y` `Value Z`)))

(event `self.ReceiveActorEndOverlap`
  (params (OtherActor :type "Actor Object Reference"))
  ;[0.15 0.15 0.15 0.5 100] Event ActorBeginOverlap
  (`/Engine/EditorBlueprintResources/StandardMacros.IsValid` OtherActor
    (:`Is Valid`
      (`|ExecutionSequence`
        (:`then_0`
          (bind _actor_of_interaction (`self.Actor Of Interaction`)
            (:`then`
              (if (== OtherActor _actor_of_interaction)
                (set `self.bFocused To Interact Actor` false)
                (set `self.bInteract In Process` false)
                (bind _hud (`self.HUD`)
                  (:`then`
                    (if (`KismetSystemLibrary.DoesImplementInterface` _hud "/Game/Core/Interfaces/BPI_HUD.BPI_HUD_C")
                      (message `/Game/Core/Interfaces/BPI_HUD.Hidden_Interact_Widget` _hud)
                      (`KismetSystemLibrary.PrintString` "Снятие фокуса и процесса взаимодействия!" true true (struct :`R` 0.991102 :`G` 0.113312 :`B` 0.156393 :`A` 1.0) 15.0)))
                  (:`else`))))
            (:`else`)))))))

(event `/Game/Core/Interfaces/BPI_Inputs.Broadcast_Camera_Zoom`
  (params (Value :type "Float (double-precision)"))
  (bind _springarm (`self.SpringArm`))
  (bind _targetarmlength (`SpringArmComponent.TargetArmLength` _springarm))
  ;[0.15 0.15 0.15 0.5 100] Приближение и отдаление камеры
  (`/Engine/EditorBlueprintResources/StandardMacros.IsValid` _springarm
    (:`Is Valid`
      (set `SpringArmComponent.TargetArmLength` (+ _targetarmlength (* (* _targetarmlength 0.05) Value)) _springarm))))

(event `/Game/Core/Interfaces/BPI_Inputs.Broadcast_Cursor_To_World`
  (params (NewLocation :type "Vector Structure") (NewRotation :type "Rotator Structure"))
  ;[0.1051 0.2606 0.6376 1 100] Отрисовка курсора в мире
  (bind _cursortoworld (`self.CursorToWorld`)
    (:`then`
      (`SceneComponent.K2_SetWorldLocationAndRotation` _cursortoworld NewLocation NewRotation false false))
    (:`else`)))

(event `/Game/Core/Interfaces/BPI_Player.Broadcast_HUD`
  (params (HUD :type "HUD Object Reference"))
  ;[0.15 0.15 0.15 0.5 100] HUD
  ;;[0.7188 0.6368 0.05886] Только Игрок
  (set `self.HUD` HUD)
  (`KismetSystemLibrary.PrintString` "Character Получил HUD" true true (struct :`R` 0.255208 :`G` 0.029178 :`B` 0.040271 :`A` 1.0) 15.0))

(event `/Game/Core/Interfaces/BPI_Inputs.Call_The_Event_Interact`
  ;[0.15 0.15 0.15 0.5 100] Interact
  (if (`self.bInteract In Process`)
    (set `self.bInteract In Process` false)
    (`self.SetActorEnableCollision` false)
    (`self.SetActorEnableCollision` true)
    (`KismetSystemLibrary.PrintString` "Взаимодействие закончено!" true true (struct :`R` 0.991102 :`G` 0.113312 :`B` 0.156393 :`A` 1.0) 15.0)
    (else
      (bind _actor_of_interaction (`self.Actor Of Interaction`)
        (:`then`
          (if (`KismetSystemLibrary.DoesImplementInterface` _actor_of_interaction "/Game/Core/Interfaces/BPI_Interactable.BPI_Interactable_C")
            (if (`self.IsOverlappingActor` _actor_of_interaction self)
              (message `/Game/Core/Interfaces/BPI_Interactable.Request_Interact` _actor_of_interaction self)
              (set `self.bInteract In Process` true))))
        (:`else`)))))

(event `/Game/Core/Interfaces/BPI_Interactable.Broadcast_Actor_Name`
  (params (Name :type Name))
  ;[0.15 0.15 0.15 0.5 100] Interact
  (if (`self.Is Player`)
    (bind _hud (`self.HUD`)
      (:`then`
        (if (`KismetSystemLibrary.DoesImplementInterface` _hud "/Game/Core/Interfaces/BPI_HUD.BPI_HUD_C")
          (message `/Game/Core/Interfaces/BPI_HUD.Update_And_Show_Interact_Widget` _hud Name)
          (`KismetSystemLibrary.PrintString` "Имя актора принято и передано в виджет!" true true (struct :`R` 0.991102 :`G` 0.113312 :`B` 0.156393 :`A` 1.0) 15.0)))
      (:`else`))))

(event `/Game/Core/Interfaces/BPI_Interactable.Broadcast_Items`
  (params (Items :type "Array of /Game/Structures/Items/F_Loot Structure (by ref)") (`Loot Actor` :type "Actor Object Reference"))
  ;[0.15 0.15 0.15 0.5 100] Interact
  (if (`self.Is Player`)
    (bind _hud (`self.HUD`)
      (:`then`
        (if (`KismetSystemLibrary.DoesImplementInterface` _hud "/Game/Core/Interfaces/BPI_HUD.BPI_HUD_C")
          (message `/Game/Core/Interfaces/BPI_HUD.Hidden_Interact_Widget` _hud)))
      (:`else`))))

(fn `Check_Player`
  (returns (IsPlayer :type Boolean))
  (return (`self.Is Player`)))

(fn `Get_Char_Direction`
  (returns (Direction :type "Float (double-precision)"))
  (bind (_returnvalue_roll _returnvalue_pitch _returnvalue_yaw) (`KismetMathLibrary.BreakRotator` (`self.K2_GetActorRotation`)))
  (return (`KismetAnimationLibrary.CalculateDirection` (`MovementComponent.Velocity` (`self.CharacterMovement`)) (`KismetMathLibrary.MakeRotator` 0.0 0.0 _returnvalue_yaw))))

(fn `Get_Char_Location`
  (returns (Location :type "Vector Structure"))
  (return (`self.K2_GetActorLocation`)))

(fn `Get_Char_Velosity_Length`
  (returns (Length :type "Float (double-precision)"))
  (return (`KismetMathLibrary.VSize` (`MovementComponent.Velocity` (`self.CharacterMovement`)))))

(fn `Get_Max_Walk_Speed`
  (returns (`Max Walk Speed` :type "Float (double-precision)"))
  (return (`CharacterMovementComponent.MaxWalkSpeed` (`self.CharacterMovement`))))

(fn `Get_State_Of_Falling`
  (returns (`Is Falling` :type Boolean))
  (return (`NavMovementInterface.IsFalling` (`self.CharacterMovement`))))

(fn `Setup Character`
  (bind _returnvalue (`self.GetController`))
  (`|ExecutionSequence`
    (:`then_0`
      (set `self.Is Player` (`KismetSystemLibrary.DoesImplementInterface` _returnvalue "/Game/Core/Interfaces/BPI_Player.BPI_Player_C"))
      ;[0.7188 0.6368 0.05886] Только Игрок
      (message `/Game/Core/Interfaces/BPI_Player.Reqest_HUD` _returnvalue self))
    (:`then_1`
      (bind _returnvalue_2 (`|AddComponentByClass` (`self.Stigmat Ref`)))
      (`/Engine/EditorBlueprintResources/StandardMacros.IsValid` _returnvalue_2
        (:`Is Valid`
          (bind _output_get (set `self.Stigmat` _returnvalue_2))
          (`/Game/Core/Components/BP_Stigmat_Component.Setup Stigmat` _output_get (`self.Start Attributes`) (`self.Start Star Blood`)))))))

(fn `UserConstructionScript`)