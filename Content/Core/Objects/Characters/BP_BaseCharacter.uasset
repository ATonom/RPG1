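; Base character with health, movement, rotation, camera zoom and a cursor-to-world marker, driven through events.
; On BeginPlay it binds to its health component, destroying itself on empty health, and spawns a Stigmata component from a class reference.
; Getters expose velocity, direction, location and falling state, and a check identifies player control through the controller's BPI_PC interface.
; Debug prints and a hit input that applies self-damage serve as test code.
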(event `/Game/Core/Interfaces/BPI_Interactable.Interact`
  (params (Message :type String))
  ;[0.04667 0.1221 0.3613 1 100] Тест
  (`KismetSystemLibrary.PrintString` Message true true (struct :`R` 1.0 :`G` 0.123894 :`B` 0.165928 :`A` 1.0) 10.0))

(event `self.ReceiveBeginPlay`
  (`|ExecutionSequence`
    (:`then_0`
      ;[0.15 0.15 0.15 0.5 100] Хелз компонент
      (bind _bp_healthcomponent (`self.BP_HealthComponent`)
        (:`then`
          (add `/Game/Core/Components/BP_Health_Component.Event On Health Empty` _bp_healthcomponent (delegate `Event On Health Empty_Event`))
          ;;[0.1144 0.3005 0.8879 1 100] Тест
          (add `/Game/Core/Components/BP_Health_Component.Event On Health Change` _bp_healthcomponent (delegate `Event On Health Change_Event`)) ; Подписываемся на изменение HP Хелз компонента
        )
        (:`else`)))
    (:`then_1`
      (`self.Setup Stigmata`))))

(event `EnhancedInput|/Game/Core/Input/Actions/IA_Hit`
  (params (ActionValue :type Boolean) (ElapsedSeconds :type "Float (double-precision)") (TriggeredSeconds :type "Float (double-precision)") (InputAction :type "InputAction Object Reference" :default "/Game/Core/Input/Actions/IA_Hit.IA_Hit"))
  ;[0.15 0.15 0.15 0.5 100] Хелз компонент
  ;;[0.1144 0.3005 0.8879 1 100] Тест
  (:`Started`
    (bind _bp_healthcomponent (`self.BP_HealthComponent`)
      (:`then`
        (`/Game/Core/Components/BP_Health_Component.Recaive Damage` _bp_healthcomponent 25.0))
      (:`else`))))

(event `Event On Health Change_Event`
  (params (`Current Health` :type "Float (double-precision)"))
  ;[0.15 0.15 0.15 0.5 100] Хелз компонент
  ;;[0.1144 0.3005 0.8879 1 100] Тест
  (`KismetSystemLibrary.PrintString` (`KismetStringLibrary.Conv_DoubleToString` `Current Health`)))

(event `Event On Health Empty_Event`
  ;[0.15 0.15 0.15 0.5 100] Хелз компонент
  (`self.K2_DestroyActor`))

(event `/Game/Core/Interfaces/BPI_Inputs.Set_Char_Rotation`
  (params (`New Rotation Z (Yaw)` :type "Float (double-precision)"))
  ;[0.15 0.15 0.15 0.5 100] Поворот персонажа
  (`self.K2_SetActorRotation` (`KismetMathLibrary.MakeRotator` 0.0 0.0 `New Rotation Z (Yaw)`)))

(event `/Game/Core/Interfaces/BPI_Inputs.Set_Move`
  (params (`Value X` :type "Float (double-precision)") (`Value Y` :type "Float (double-precision)") (`Value Z` :type "Float (double-precision)"))
  ;[0.15 0.15 0.15 0.5 100] Передвижение
  (`self.AddMovementInput` (`KismetMathLibrary.MakeVector` `Value X` `Value Y` `Value Z`)))

(event `/Game/Core/Interfaces/BPI_Inputs.Set_Cursor_To_World`
  (params (NewLocation :type "Vector Structure") (NewRotation :type "Rotator Structure"))
  ;[0.15 0.15 0.15 0.5 100] Положение курсора в мире
  (bind _cursortoworld (`self.CursorToWorld`)
    (:`then`
      (`SceneComponent.K2_SetWorldLocationAndRotation` _cursortoworld NewLocation NewRotation false false))
    (:`else`)))

(event `/Game/Core/Interfaces/BPI_Inputs.Set_Camera_Zoom`
  (params (Value :type "Float (double-precision)"))
  (bind _springarm (`self.SpringArm`))
  (bind _targetarmlength (`SpringArmComponent.TargetArmLength` _springarm))
  ;[0.15 0.15 0.15 0.5 100] Приближение и отдаление камеры
  (set `SpringArmComponent.TargetArmLength` (+ _targetarmlength (* (* _targetarmlength 0.05) Value)) _springarm))

(fn `Check_Player`
  (returns (IsPlayer :type Boolean))
  (return (`KismetSystemLibrary.DoesImplementInterface` (`self.GetController`) "/Game/Core/Interfaces/BPI_PC.BPI_PC_C")))

(fn `Get_Char_Direction`
  (returns (Direction :type "Float (double-precision)"))
  (bind (_returnvalue_roll _returnvalue_pitch _returnvalue_yaw) (`KismetMathLibrary.BreakRotator` (`self.K2_GetActorRotation`)))
  (return (`KismetAnimationLibrary.CalculateDirection` (`MovementComponent.Velocity` (`self.CharacterMovement`)) (`KismetMathLibrary.MakeRotator` 0.0 0.0 _returnvalue_yaw))))

(fn `Get_Char_Location`
  (returns (Location :type "Vector Structure"))
  (return (`self.K2_GetActorLocation`)))

(fn `Get_Char_Velosity_Length`
  (returns (Length :type "Float (double-precision)"))
  (return (`KismetMathLibrary.VSize` (`MovementComponent.Velocity` (`self.CharacterMovement`)))))

(fn `Get_Max_Walk_Speed`
  (returns (`Max Walk Speed` :type "Float (double-precision)"))
  (return (`CharacterMovementComponent.MaxWalkSpeed` (`self.CharacterMovement`))))

(fn `Get_State_Of_Falling`
  (returns (`Is Falling` :type Boolean))
  (return (`NavMovementInterface.IsFalling` (`self.CharacterMovement`))))

(fn `Setup Stigmata`
  (bind _returnvalue (`|AddComponentByClass` (`self.Stigmata Ref`)))
  (`/Engine/EditorBlueprintResources/StandardMacros.IsValid` _returnvalue
    (:`Is Valid`
      (bind _output_get (set `self.Stigmata` _returnvalue))
      (`/Game/Core/Components/BP_Stigmata_Component.Setup Stigmata` _output_get))))

(fn `UserConstructionScript`)