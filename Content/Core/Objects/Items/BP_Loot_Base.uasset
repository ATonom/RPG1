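; BP_Loot_Base is a base loot actor that hands its name and item list to an interacting player.
; Name and interact requests pass through IsPlayerInteract, which checks the BPI_Interactable and BPI_Player interfaces, then calls CheckPlayerMessage.
; Valid players receive ActorName or the Loot array with a self reference via interface messages, alongside debug prints.
; BeginPlay and Collect are empty stubs, with mesh loading and array filling noted as rework.
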(event `/Game/Core/Interfaces/BPI_Interactable.Request_Actor_Name`
  (params (`Other Actor` :type "Actor Object Reference"))
  ;[0.1051 0.2606 0.6376 1 100] BPI Intetactable
  (`/Engine/EditorBlueprintResources/StandardMacros.IsValid` `Other Actor`
    (:`Is Valid`
      (bind _isplayer (`self.Is Player interact` `Other Actor`))
      (if _isplayer
        (message `/Game/Core/Interfaces/BPI_Interactable.Broadcast_Actor_Name` `Other Actor` (`self.Actor Name`))
        (`KismetSystemLibrary.PrintString` "Имя передано!" true true (struct :`R` 0.159759 :`G` 1.0 :`B` 0.073619 :`A` 1.0) 15.0)
        (else
          (`/Engine/EditorBlueprintResources/StandardMacros.DoOnce` false
            (:`Completed`
              (`KismetSystemLibrary.PrintString` "Имя не передано!" true true (struct :`R` 0.158961 :`G` 0.991102 :`B` 0.074214 :`A` 1.0) 15.0))))))))

(event `self.ReceiveBeginPlay`
  ;[0.1051 0.2606 0.6376 1 50] Переделать
  ; - Загрузка Mesh
  ; - Заполнение массива придметов
)

(event `/Game/Core/Interfaces/BPI_Interactable.Request_Interact`
  (params (`Other Actor` :type "Actor Object Reference"))
  ;[0.1051 0.2606 0.6376 1 100] BPI Intetactable
  (`/Engine/EditorBlueprintResources/StandardMacros.IsValid` `Other Actor`
    (:`Is Valid`
      (bind _isplayer (`self.Is Player interact` `Other Actor`))
      (if _isplayer
        (message `/Game/Core/Interfaces/BPI_Interactable.Broadcast_Items` `Other Actor` (`self.Loot`) self)
        (`KismetSystemLibrary.PrintString` "Перечень предметов передан Игроку!" true true (struct :`R` 0.159759 :`G` 1.0 :`B` 0.073619 :`A` 1.0) 15.0)))))

(event `/Game/Core/Interfaces/BPI_Interactable.Collect`
  ;[0.1051 0.2606 0.6376 1 100] BPI Intetactable
)

(fn `Is Player interact`
  (params (Actor :type "Object Object Reference"))
  (returns (IsPlayer :type Boolean))
  (if (`KismetSystemLibrary.DoesImplementInterface` Actor "/Game/Core/Interfaces/BPI_Interactable.BPI_Interactable_C")
    (if (`KismetSystemLibrary.DoesImplementInterface` Actor "/Game/Core/Interfaces/BPI_Player.BPI_Player_C")
      (bind _isplayer (message `/Game/Core/Interfaces/BPI_Player.Check_Player` Actor))
      (return _isplayer))))

(fn `UserConstructionScript`)