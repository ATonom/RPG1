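; BP_Item_Rune is a pickup rune item whose mesh material reflects its Tier.
; SetupMaterial looks up the tier's row in DT_Item_Runes_Info and applies its material, both at construction and on BeginPlay.
; Interact verifies the other actor through BPI_Interactable and BPI_Player, then sends it type, ID, quantity and itself via BroadcastItemMessage.
; A separate Collect event destroys the rune, with debug prints tracing the pickup.
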(event `self.ReceiveBeginPlay`
  ;[0.03337 0.4678 0.01398 1 50] Перенести в Руну
  (`self.Setup Material`))

(event `/Game/Core/Interfaces/BPI_Interactable.Interact`
  (params (`Qther Actor` :type "Actor Object Reference"))
  ;[0.1051 0.2606 0.6376 1 100] Подбор предмета
  (`|ExecutionSequence`
    (:`then_0`
      (if (`KismetSystemLibrary.DoesImplementInterface` `Qther Actor` "/Game/Core/Interfaces/BPI_Interactable.BPI_Interactable_C")
        (if (`KismetSystemLibrary.DoesImplementInterface` `Qther Actor` "/Game/Core/Interfaces/BPI_Player.BPI_Player_C")
          (bind _isplayer (message `/Game/Core/Interfaces/BPI_Player.Check_Player` `Qther Actor`))
          (if _isplayer
            (message `/Game/Core/Interfaces/BPI_Interactable.Broadcast Item` `Qther Actor` (`self.Type`) (`self.ID`) (`self.Quantity`) self)
            (`KismetSystemLibrary.PrintString` "Данные переданы" true true (struct :`R` 0.159759 :`G` 1.0 :`B` 0.073619 :`A` 1.0) 15.0)
            (else
              (`/Engine/EditorBlueprintResources/StandardMacros.DoOnce` false
                (:`Completed`
                  (`KismetSystemLibrary.PrintString` "Это не игрок!" true true (struct :`R` 0.158961 :`G` 0.991102 :`B` 0.074214 :`A` 1.0) 15.0))))))))))

(event `/Game/Core/Interfaces/BPI_Interactable.Collect`
  ;[0.1051 0.2606 0.6376 1 100] Подбор предмета
  (`KismetSystemLibrary.PrintString` "Предмет уничтожен!" true true (struct :`R` 0.158961 :`G` 0.991102 :`B` 0.074214 :`A` 1.0) 15.0)
  (`self.K2_DestroyActor`))

(fn `Broadcast Item`
  (params (Type :type "/Game/Enums/E_Item_Type Enum" :default "NewEnumerator0") (ID :type Integer) (Quantity :type Integer) (`Item Actor` :type "Actor Object Reference")))

(fn `Setup Material`
  (bind _returnvalue (`|GetDataTableRow` "/Game/Tables/DT_Item_Runes_Info.DT_Item_Runes_Info" (`KismetStringLibrary.Conv_StringToName` (`|GetEnumeratorNameAsString` (`self.Tier`))))
    (:`then`
      (`PrimitiveComponent.SetMaterial` (`self.Mesh`) 0 (`.RuneMaterial_6_AD3C1941488CE957239609B37CC2E690` (break `/Game/Structures/Rune/F_Item_Rune_Info` _returnvalue))))))

(fn `UserConstructionScript`
  (`self.Setup Material`))