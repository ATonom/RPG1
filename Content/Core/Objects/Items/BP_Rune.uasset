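; BP_Rune is a collectible rune item whose mesh material reflects its tier.
; SetupMaterial looks up the tier name in DT_Runes_Info and applies that row's material, both in the construction script and at BeginPlay.
; On overlap with an actor implementing both the interactable and player character interfaces, it runs that actor's message check, sends a collected message and destroys itself.
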(event `self.ReceiveBeginPlay`
  (`self.Setup Material`))

(event `self.ReceiveActorBeginOverlap`
  (params (OtherActor :type "Actor Object Reference"))
  (if (`KismetSystemLibrary.DoesImplementInterface` OtherActor "/Game/Core/Interfaces/BPI_Interactable.BPI_Interactable_C")
    (if (`KismetSystemLibrary.DoesImplementInterface` OtherActor "/Game/Core/Interfaces/BPI_Player_Char.BPI_Player_Char_C")
      (bind _isplayer (message `/Game/Core/Interfaces/BPI_Player_Char.Check_Player` OtherActor))
      (if _isplayer
        ;[0.1051 0.2606 0.6376 1 100] Тест
        (message `/Game/Core/Interfaces/BPI_Interactable.Interact` OtherActor "The rune is collected!")
        (`self.K2_DestroyActor`)))))

(fn `Setup Material`
  (bind _returnvalue (`|GetDataTableRow` "/Game/Tables/DT_Runes_Info.DT_Runes_Info" (`KismetStringLibrary.Conv_StringToName` (`|GetEnumeratorNameAsString` (`self.Tier`))))
    (:`then`
      (`PrimitiveComponent.SetMaterial` (`self.Mesh`) 0 (`.RuneMaterial_6_AD3C1941488CE957239609B37CC2E690` (break `/Game/Structures/Rune/F_Rune_Info` _returnvalue))))))

(fn `UserConstructionScript`
  (`self.Setup Material`))