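; Base player controller for a cursor-aimed character, adding the default Enhanced Input mapping and showing the mouse.
; Move, zoom and interact inputs go to the pawn through the BPI_Inputs interface, with movement scaled by max walk speed.
; Each tick, a cursor trace turns the character toward the hit and aligns a world cursor to the surface normal.
; It also caches the HUD and passes it to requesting actors.
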(event `self.ReceiveBeginPlay`
  (bind _returnvalue (subsystem `EnhancedInputLocalPlayerSubsystem`))
  (`|ExecutionSequence`
    (:`then_0`
      ;[0.15 0.15 0.15 0.5 100] Add Mapping Context
      (`/Engine/EditorBlueprintResources/StandardMacros.IsValid` _returnvalue
        (:`Is Valid`
          (message `EnhancedInputSubsystemInterface.AddMappingContext` _returnvalue "/Game/Core/Input/IMC_Default.IMC_Default" 0 (struct))
          (set `self.bShowMouseCursor` true))))
    (:`then_1`
      (set `self.HUD` (`self.GetHUD`)))))

(event `EnhancedInput|/Game/Core/Input/Actions/IA_Move`
  (params (ActionValue :type "Vector2D Structure") (ElapsedSeconds :type "Float (double-precision)") (TriggeredSeconds :type "Float (double-precision)") (InputAction :type "InputAction Object Reference" :default "/Game/Core/Input/Actions/IA_Move.IA_Move"))
  ;[0.15 0.15 0.15 0.5 100] IA Move
  (:`Triggered`
    (`self.Move` ActionValue)))

(event `/Game/Core/Interfaces/BPI_Player.Reqest_HUD`
  (params (`Other Actor` :type "Actor Object Reference"))
  ;[0.15 0.15 0.15 0.5 100] HUD
  (message `/Game/Core/Interfaces/BPI_Player.Broadcast_HUD` `Other Actor` (`self.HUD`)))

(event `self.ReceiveTick`
  (params (DeltaSeconds :type "Float (single-precision)"))
  (bind (_hit _location _impact_normal) (`self.GetLocationUnderCursor`))
  ;[0.15 0.15 0.15 0.5 100] Поворот персонажа и положения курсора в мире
  (if _hit
    (`self.Set Character Rotation` _location)
    (`self.Set Location and Rotation Cursor To World` _location _impact_normal)))

(event `EnhancedInput|/Game/Core/Input/Actions/IA_Interact`
  (params (ActionValue :type Boolean) (ElapsedSeconds :type "Float (double-precision)") (TriggeredSeconds :type "Float (double-precision)") (InputAction :type "InputAction Object Reference" :default "/Game/Core/Input/Actions/IA_Interact.IA_Interact"))
  ;[0.15 0.15 0.15 0.5 100] IA Interact
  (:`Canceled`
    (`self.Interact` :!label _label))
  (:`Completed`
    (goto _label)))

(event `EnhancedInput|/Game/Core/Input/Actions/IA_CameraZoom`
  (params (ActionValue :type "Float (double-precision)") (ElapsedSeconds :type "Float (double-precision)") (TriggeredSeconds :type "Float (double-precision)") (InputAction :type "InputAction Object Reference" :default "/Game/Core/Input/Actions/IA_CameraZoom.IA_CameraZoom"))
  ;[0.15 0.15 0.15 0.5 100] IA CameraZoom
  (:`Triggered`
    (`self.Camera Zoom` ActionValue)))

(event `EnhancedInput|/Game/Core/Input/Actions/IA_Hit`
  (params (ActionValue :type Boolean) (ElapsedSeconds :type "Float (double-precision)") (TriggeredSeconds :type "Float (double-precision)") (InputAction :type "InputAction Object Reference" :default "/Game/Core/Input/Actions/IA_Hit.IA_Hit")))

(fn `Camera Zoom`
  (params (Value :type "Float (double-precision)"))
  (bind _returnvalue (`GameplayStatics.GetPlayerPawn` 0))
  (if (`KismetSystemLibrary.DoesImplementInterface` _returnvalue "/Game/Core/Interfaces/BPI_Inputs.BPI_Inputs_C")
    (message `/Game/Core/Interfaces/BPI_Inputs.Broadcast_Camera_Zoom` _returnvalue Value)))

(fn `Check_Player`
  (returns (IsPlayer :type Boolean))
  (return true))

(fn `GetLocationUnderCursor`
  (returns (Hit :type Boolean) (Location :type "Vector Structure") (`Impact Normal` :type "Vector Structure"))
  (bind (_bblockinghit _binitialoverlap _time _distance _location _impactpoint _normal _impactnormal) (`GameplayStatics.BreakHitResult` (`self.GetHitResultUnderCursorByChannel` "TraceTypeQuery3")))
  (return _bblockinghit _location _impactnormal))

(fn `Interact`
  (bind _returnvalue (`GameplayStatics.GetPlayerPawn` 0))
  (if (`KismetSystemLibrary.DoesImplementInterface` _returnvalue "/Game/Core/Interfaces/BPI_Inputs.BPI_Inputs_C")
    (message `/Game/Core/Interfaces/BPI_Inputs.Call_The_Event_Interact` _returnvalue)))

(fn `Move`
  (params (`Action Vector` :type "Vector2D Structure"))
  (bind _returnvalue (`GameplayStatics.GetPlayerPawn` 0))
  (if (`KismetSystemLibrary.DoesImplementInterface` _returnvalue "/Game/Core/Interfaces/BPI_Inputs.BPI_Inputs_C")
    ;[0.1051 0.2606 0.6376] В дальнейшем нужно заменить на Current speed
    (bind _max_walk_speed (message `/Game/Core/Interfaces/BPI_Inputs.Get_Max_Walk_Speed` _returnvalue))
    (message `/Game/Core/Interfaces/BPI_Inputs.Broadcast_Move` _returnvalue (* _max_walk_speed `Action Vector_X`) (* _max_walk_speed `Action Vector_Y`) 0.0)))

(fn `Set Character Rotation`
  (params (Location :type "Vector Structure"))
  (bind _returnvalue (`GameplayStatics.GetPlayerPawn` 0))
  (if (`KismetSystemLibrary.DoesImplementInterface` _returnvalue "/Game/Core/Interfaces/BPI_Inputs.BPI_Inputs_C")
    (bind _location (message `/Game/Core/Interfaces/BPI_Inputs.Get_Char_Location` _returnvalue))
    (bind (_returnvalue_roll _returnvalue_pitch _returnvalue_yaw) (`KismetMathLibrary.BreakRotator` (`KismetMathLibrary.FindLookAtRotation` _location Location)))
    (message `/Game/Core/Interfaces/BPI_Inputs.Broadcast_Char_Rotation` _returnvalue _returnvalue_yaw)))

(fn `Set Location and Rotation Cursor To World`
  (params (Location :type "Vector Structure") (`Inpact Normal` :type "Vector Structure"))
  (bind _returnvalue (`GameplayStatics.GetPlayerPawn` 0))
  (if (`KismetSystemLibrary.DoesImplementInterface` _returnvalue "/Game/Core/Interfaces/BPI_Inputs.BPI_Inputs_C")
    (message `/Game/Core/Interfaces/BPI_Inputs.Broadcast_Cursor_To_World` _returnvalue Location (`KismetMathLibrary.Conv_VectorToRotator` `Inpact Normal`))))

(fn `UserConstructionScript`)