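; BP_Characteristic wraps a single Characteristic struct that holds a value, a parent key and child keys, linking it to related characteristics.
; A setup function stores the struct, and getters expose each of its three fields.
; Child keys are appended individually, while AddValue increments the value and then reassigns the struct from that value with a None parent key.
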(fn `Add Child Key`
  (params (`Child Key` :type Name))
  (bind (_characteristic_value _characteristic_parentkey _characteristic_childkeys) (break `/Game/Structures/Characteristics/F_Characteristic` (`self.Characteristic`)))
  (`KismetArrayLibrary.Array_Add` _characteristic_childkeys `Child Key`))

(fn `Add Value`
  (bind _characteristic_value (break `/Game/Structures/Characteristics/F_Characteristic` (`self.Characteristic`)))
  (`/Engine/EditorBlueprintResources/StandardMacros.IncrementInt` _characteristic_value
    (:`  `
      (set `self.Characteristic` (make `/Game/Structures/Characteristics/F_Characteristic` _characteristic_value)))))

(fn `Get Child Keys`
  (returns (`Child Keys` :type "Array of Name"))
  (bind (_characteristic_value _characteristic_parentkey _characteristic_childkeys) (break `/Game/Structures/Characteristics/F_Characteristic` (`self.Characteristic`)))
  (return _characteristic_childkeys))

(fn `Get Parent Key`
  (returns (`Parent Key` :type Name))
  (bind (_characteristic_value _characteristic_parentkey) (break `/Game/Structures/Characteristics/F_Characteristic` (`self.Characteristic`)))
  (return _characteristic_parentkey))

(fn `Get Value`
  (returns (Value :type Integer))
  (bind _characteristic_value (break `/Game/Structures/Characteristics/F_Characteristic` (`self.Characteristic`)))
  (return _characteristic_value))

(fn `Setup Characteristic`
  (params (Characteristic :type "/Game/Structures/Characteristics/F_Characteristic Structure"))
  (set `self.Characteristic` Characteristic))