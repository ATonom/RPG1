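; Attributes manager component that loads attribute definitions and maximums from two data tables on BeginPlay.
; Info rows form an index-linked hierarchy: each added entry registers itself in its parent's child list in the same pass, so it relies on parents preceding children.
; Max rows fill a separate array, and the attribute count is cached for a getter.
; A Test function prints each attribute with its tier, parent and children.
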(event `self.ReceiveBeginPlay`
  (`self.Setup Attributes Info from DT`)
  (`self.Setup Attributes Max from DT`)
  (set `self.Number Of Attributes` (`KismetArrayLibrary.Array_Length` (`self.Attributes Info`))))

(fn `Get Number Of Attributes`
  (returns (`Number Of Attributes` :type Integer))
  (return (`self.Number Of Attributes`)))

(fn `Setup Attributes Info from DT`
  (bind _attributes_info (`self.Attributes Info`))
  (bind _outrownames (`DataTableFunctionLibrary.GetDataTableRowNames` "/Game/Tables/DT_Attributes_Info.DT_Attributes_Info"))
  (for _array_element _outrownames
    (bind _returnvalue (`|GetDataTableRow` "/Game/Tables/DT_Attributes_Info.DT_Attributes_Info" _array_element)
      (:`then`
        (bind _returnvalue_2 (`KismetArrayLibrary.Array_Add` _attributes_info _returnvalue))
        (bind (_output_name _output_tier _output_parentindex) (break `/Game/Structures/Attributes/F_Attribute_info` (`|GetArrayItem` _attributes_info _returnvalue_2)))
        (bind (_output_name_2 _output_tier_2 _output_parentindex_2 _output_childindexes) (break `/Game/Structures/Attributes/F_Attribute_info` (`|GetArrayItem` _attributes_info _output_parentindex)))
        (`KismetArrayLibrary.Array_Add` _output_childindexes _returnvalue_2)))))

(fn `Setup Attributes Max from DT`
  (bind _outrownames (`DataTableFunctionLibrary.GetDataTableRowNames` "/Game/Tables/DT_Attributes_Max.DT_Attributes_Max"))
  (for _array_element _outrownames
    (bind _returnvalue (`|GetDataTableRow` "/Game/Tables/DT_Attributes_Max.DT_Attributes_Max" _array_element)
      (:`then`
        (`KismetArrayLibrary.Array_Add` (`self.Attributes Max`) _returnvalue)))))

(fn `Test`
  (locals (NewLocalVar :type String))
  (bind _newlocalvar (`local.NewLocalVar`))
  (for (_array_element _array_index) (`self.Attributes Info`)
    (set `local.NewLocalVar` (`KismetStringLibrary.Concat_StrStr` (`KismetStringLibrary.Conv_IntToString` _array_index) " / " (`KismetTextLibrary.Conv_TextToString` (break `/Game/Structures/Attributes/F_Attribute_info` _array_element)) " / " (`|GetEnumeratorNameAsString` (`.Tier_9_030B4CD04A0913CCFB42C089219222F8` (break `/Game/Structures/Attributes/F_Attribute_info` _array_element))) " / " (`KismetStringLibrary.Conv_IntToString` (`.ParentIndex_26_0451902F4705B3A9B91822B93ADFF518` (break `/Game/Structures/Attributes/F_Attribute_info` _array_element))) " / " (`KismetTextLibrary.Conv_TextToString` (`.Description_17_05651B294B87EDE7795412B1D2142AEF` (break `/Game/Structures/Attributes/F_Attribute_info` _array_element)))))
    (for _array_element_2 (`.ChildIndexes_27_200992324AAB3F3B796E86965414ACE1` (break `/Game/Structures/Attributes/F_Attribute_info` _array_element))
      (set `local.NewLocalVar` (`KismetStringLibrary.Concat_StrStr` _newlocalvar " / " (`KismetStringLibrary.Conv_IntToString` _array_element_2))))
    (`KismetSystemLibrary.PrintString` _newlocalvar true true (struct :`G` 0.66 :`B` 1.0 :`A` 1.0) 20.0)))