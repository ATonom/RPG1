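; Health component that tracks current and maximum health for its owning actor, starting at full on BeginPlay.
; RecaiveDamage subtracts damage, clamps health at zero and fires the OnHealthEmpty event when depleted, then always broadcasts OnHealthChange with the new value.
; The empty event fires before the change event and repeats on further hits at zero.
; Getters expose current and maximum health.
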(event `self.ReceiveBeginPlay`
  (set `self.Current Health` (`self.Max Health`)))

(fn `Get Current Health`
  (returns (`Current Health` :type "Float (double-precision)"))
  (return (`self.Current Health`)))

(fn `Get Max Health`
  (returns (`Current Health` :type "Float (double-precision)"))
  (return (`self.Max Health`)))

(fn `Recaive Damage`
  (params (Damage :type "Float (double-precision)"))
  (set `self.Current Health` (- (`self.Current Health`) Damage))
  (`|ExecutionSequence`
    (:`then_0`
      (if (<= (`self.Current Health`) 0.0)
        (set `self.Current Health` 0.0)
        (`self.Event On Health Empty`)))
    (:`then_1`
      (`self.Event On Health Change` (`self.Current Health`)))))