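; Stigmat actor component that holds its owner's attribute array, StarBlood pool and capped list of runes.
; On BeginPlay it caches the owner, requests the attribute count from the GameMode through BPI_Attributes_Manager, and sets StarBlood to its maximum.
; SetupStigmat zero-pads attributes to that count, overlays starting values and initializes StarBlood.
; AddMaxStarBlood sets the maximum to current StarBlood plus the given value.
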(event `self.ReceiveBeginPlay`
  ;[0.15 0.15 0.15 0.502 50] Event Begin Play
  (`|ExecutionSequence`
    (:`then_0`
      (set `self.Сharacter` (`self.GetOwner`)))
    (:`then_1`
      (`self.Requesting Data For Setuping`))
    (:`then_2`
      (set `self.Star Blood` (`self.Max Star Blood`)))))

(event `/Game/Core/Interfaces/BPI_Attributes_Manager.Broadcast_Number_Of_Attributes`
  (params (`Number Of Attributes` :type Integer))
  ;[0.15 0.15 0.15 0.502 50] Event Begin Play
  (set `self.Number Of Attributes` `Number Of Attributes`))

(fn `Add Max Star Blood`
  (params (Value :type "Float (double-precision)"))
  (set `self.Max Star Blood` (+ Value (`self.Star Blood`))))

(fn `Add Rune`
  (params (`New Rune` :type "/Game/Structures/Runes/F_Rune_Info Structure (by ref)"))
  (`KismetArrayLibrary.Array_Add` (`self.Runes`) `New Rune`))

(fn `Check Free Runes Slot`
  (returns (`Rune Bag Is Not Full` :type Boolean))
  (return (> (`self.Max Number Of Runes`) (`KismetArrayLibrary.Array_Length` (`self.Runes`)))))

(fn `Request_Number_Of_Attributes`
  (params (`Requesting Objest` :type "Object Object Reference"))
  (return))

(fn `Requesting Data For Setuping`
  (bind _returnvalue (`GameplayStatics.GetGameMode`))
  (`|ExecutionSequence`
    (:`then_0`
      (`/Engine/EditorBlueprintResources/StandardMacros.IsValid` _returnvalue
        (:`Is Valid`
          (if (`KismetSystemLibrary.DoesImplementInterface` _returnvalue "/Game/Core/Interfaces/BPI_Attributes_Manager.BPI_Attributes_Manager_C")
            (message `/Game/Core/Interfaces/BPI_Attributes_Manager.Request_Number_Of_Attributes` _returnvalue self)))))))

(fn `Setup Attributes`
  (params (`Start Attributes` :type "Array of /Game/Structures/Attributes/F_Attribute Structure"))
  (bind _attributes (`self.Attributes`))
  (`|ExecutionSequence`
    (:`then_0`
      (`/Engine/EditorBlueprintResources/StandardMacros.Do N` (`self.Number Of Attributes`) :!label _label
        (:`Exit`
          (`KismetArrayLibrary.Array_Add` (`self.Attributes`))
          (goto _label))))
    (:`then_1`
      (for _array_element `Start Attributes`
        (if (`KismetArrayLibrary.Array_IsValidIndex` _attributes (break `/Game/Structures/Attributes/F_Attribute` _array_element))
          (`KismetArrayLibrary.Array_Set` _attributes (break `/Game/Structures/Attributes/F_Attribute` _array_element) (`.Value_4_A3BC46BD49B12C2415518D91D2F0C7EE` (break `/Game/Structures/Attributes/F_Attribute` _array_element))))))))

(fn `Setup Stigmat`
  (params (`Start Attributes` :type "Array of /Game/Structures/Attributes/F_Attribute Structure") (`Start Star Blood` :type "Float (double-precision)"))
  (`self.Setup Attributes` `Start Attributes`)
  (`self.Add Max Star Blood` `Start Star Blood`)
  (set `self.Star Blood` `Start Star Blood`))