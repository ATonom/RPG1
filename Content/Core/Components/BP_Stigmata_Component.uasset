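; Stigmata component that builds a hierarchy of characteristic objects from the DT_Characteristics_Info data table.
; Setup creates one object per row at zero value with its parent key, storing it in CharacteristicsMap by row name.
; Each new object registers as a child of its parent only if that parent is already mapped, so row order matters.
; A Test function prints each characteristic's name, tier and parent name.
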(event `self.ReceiveBeginPlay`)

(fn `Setup Characteristics from DT`
  (bind _outrownames (`DataTableFunctionLibrary.GetDataTableRowNames` "/Game/Tables/DT_Characteristics_Info.DT_Characteristics_Info"))
  (for _array_element _outrownames
    ;[0.15 0.15 0.15 0.5 50] Добавление новой харастеристики
    (bind _returnvalue (`|GetDataTableRow` "/Game/Tables/DT_Characteristics_Info.DT_Characteristics_Info" _array_element)
      (:`then`
        (bind _returnvalue_2 (`|GenericCreateObject` (`self.Characteristic Ref`)))
        (`/Engine/EditorBlueprintResources/StandardMacros.IsValid` _returnvalue_2
          (:`Is Valid`
            (`/Game/Core/Components/BP_Characteristic.Setup Characteristic` _returnvalue_2 (make `/Game/Structures/Characteristics/F_Characteristic` 0 (`.ParentKey_19_0451902F4705B3A9B91822B93ADFF518` (break `/Game/Structures/Characteristics/F_Characteristic_Info` _returnvalue))))
            (`BlueprintMapLibrary.Map_Add` (`self.Characteristics Map`) _array_element _returnvalue_2)
            (bind (_value _returnvalue_3) (`BlueprintMapLibrary.Map_Find` (`self.Characteristics Map`) (`.ParentKey_19_0451902F4705B3A9B91822B93ADFF518` (break `/Game/Structures/Characteristics/F_Characteristic_Info` _returnvalue))))
            ;[0.15 0.15 0.15 0.5 50] Регистрация дочерней характиристики
            (if _returnvalue_3
              (`/Game/Core/Components/BP_Characteristic.Add Child Key` _value _array_element))))))))

(fn `Setup Stigmata`
  (`self.Setup Characteristics from DT`))

(fn `Test`
  (bind _outrownames (`DataTableFunctionLibrary.GetDataTableRowNames` "/Game/Tables/DT_Characteristics_Info.DT_Characteristics_Info"))
  (for _array_element _outrownames
    (bind (_value _returnvalue) (`BlueprintMapLibrary.Map_Find` (`self.Characteristics Map`) _array_element))
    (if _returnvalue
      (bind _parent_key (`/Game/Core/Components/BP_Characteristic.Get Parent Key` _value))
      (bind _returnvalue_2 (`|GetDataTableRow` "/Game/Tables/DT_Characteristics_Info.DT_Characteristics_Info" _parent_key)
        (:`then`
          _)
        (:`RowNotFound`
          _))
      (bind _returnvalue_3 (`|GetDataTableRow` "/Game/Tables/DT_Characteristics_Info.DT_Characteristics_Info" _array_element)
        (:`then`
          _)
        (:`RowNotFound`
          _))
      (`KismetSystemLibrary.PrintString` (`KismetStringLibrary.Concat_StrStr` (`KismetTextLibrary.Conv_TextToString` (break `/Game/Structures/Characteristics/F_Characteristic_Info` _returnvalue_3)) "-[" (`|GetEnumeratorNameAsString` (`.Tier_9_030B4CD04A0913CCFB42C089219222F8` (break `/Game/Structures/Characteristics/F_Characteristic_Info` _returnvalue_3))) "]-" (`KismetTextLibrary.Conv_TextToString` (break `/Game/Structures/Characteristics/F_Characteristic_Info` _returnvalue_2))) true true (struct :`G` 0.66 :`B` 1.0 :`A` 1.0) 10.0))))